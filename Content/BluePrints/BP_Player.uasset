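; BP_Player is the player character Blueprint, handling movement, camera look, jumping and health pickups.
; Input axes move it along the capsule's forward and right vectors and add controller yaw and pitch, while the Jump action triggers the standard character jump.
; An IncreaseHealth event adds the given amount to Health and caps it at a maximum.
; BeginPlay and the Respawn event are empty.
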(event Custom|Increase%20Health
  (params (Add%20health :type Float%20%28double-precision%29))
  ;[0.15 0.15 0.15 0.5] Health Pickup
  (Variables|Default|SetHealth (+ (Variables|Default|GetHealth) Add%20health))
  (if (> (Variables|Default|GetHealth) 1e+02)
    (Variables|Default|SetHealth 1e+02)))

(event Custom|Respawn)

(event EventBeginPlay)

(event Input|ActionEvents|InputActionJump
  (params (Key :type Key%20Structure :default "None"))
  ;[0.15 0.15 0.15 0.5] Action Mapping
  (:Pressed
    (Character|Jump)))

(event Input|AxisEvents|InputAxisTurn
  (params (AxisValue :type Float%20%28single-precision%29))
  ;[0.15 0.15 0.15 0.5] Camera
  (Pawn|Input|AddControllerYawInput AxisValue))

(event Input|AxisEvents|InputAxisLookUp
  (params (AxisValue :type Float%20%28single-precision%29))
  ;[0.15 0.15 0.15 0.5] Camera
  (Pawn|Input|AddControllerPitchInput AxisValue))

(event Input|AxisEvents|InputAxisMove_Forward
  (params (AxisValue :type Float%20%28single-precision%29))
  ;[0.15 0.15 0.15 0.5] Movement
  (Pawn|Input|AddMovementInput (Math|Vector|GetForwardVector (Variables|Collision|GetCapsuleComponent)) AxisValue false))

(event Input|AxisEvents|InputAxisMove_Right
  (params (AxisValue :type Float%20%28single-precision%29))
  ;[0.15 0.15 0.15 0.5] Movement
  (Pawn|Input|AddMovementInput (Math|Vector|GetRightVector (Variables|Collision|GetCapsuleComponent)) AxisValue false))

(fn ConstructionScript)