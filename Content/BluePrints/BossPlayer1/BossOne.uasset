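; BossOne is a boss pawn Blueprint that moves through an array of waypoint actors using AI navigation.
; On BeginPlay it calls Chase, which runs AI MoveTo toward the current waypoint.
; Each successful move increments the index, resets it to zero only once it exceeds the array length, and calls Chase again.
; Failed moves have no handling.
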(event Custom|Chase
  ;[0.15 0.15 0.15 0.5] WayPoints
  (AI|AIMoveTo self "0, 0, 0" (Utilities|Array|Get(acopy) (Variables|Default|GetWayPoints) (Variables|Default|GetcurrentWayPoint)) 5.0 false
    (:OnSuccess
      (Math|Integer|IncrementInt (Variables|Default|GetcurrentWayPoint)
        (:%20%20
          (if (> (Variables|Default|GetcurrentWayPoint) (Utilities|Array|Length (Variables|Default|GetWayPoints)))
            (Variables|Default|SetcurrentWayPoint 0))
          (CallFunction|Chase))))))

(event EventBeginPlay
  (CallFunction|Chase))

(fn ConstructionScript)