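; BossEnemy1 is a boss enemy pawn that patrols an array of waypoint actors in an endless loop.
; BeginPlay starts the waypoint event, which uses AI MoveTo toward the current waypoint.
; On success it advances the index, wraps to zero past the last entry and re-triggers itself.
; Debug strings print "sucess" on wrap and "fail" on ordinary advances, while failed moves have no handling.
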(event Custom|Follow_Waypoints
  (AI|AIMoveTo self "0, 0, 0" (Utilities|Array|Get(acopy) (Variables|Default|GetWayPoints) (Variables|Default|GetCurrent)) 5.0 false
    (:OnSuccess
      (Math|Integer|IncrementInt (Variables|Default|GetCurrent)
        (:%20%20
          (if (>= (Variables|Default|GetCurrent) (Utilities|Array|Length (Variables|Default|GetWayPoints)))
            (Development|PrintString "sucess")
            (Variables|Default|SetCurrent 0)
            (else
              (Development|PrintString "fail")))
          (CallFunction|FollowWaypoints))))))

(event EventBeginPlay
  (CallFunction|FollowWaypoints))

(fn ConstructionScript)