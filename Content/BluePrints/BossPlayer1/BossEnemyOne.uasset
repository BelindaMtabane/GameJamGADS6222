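; BossEnemyOne is a boss enemy that patrols a looping route of waypoints.
; From BeginPlay, ChasePlayer uses AIMoveTo toward the current waypoint actor; despite its name, it never targets the player.
; On success it advances the index, wrapping to the first waypoint, waits briefly and calls itself again.
; A failed move is not handled, so the patrol stops there.
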(event Custom|ChasePlayer
  (AI|AIMoveTo self "0, 0, 0" (Utilities|Array|Get(acopy) (Variables|Default|GetwayPoints) (Variables|Default|GetCurrentWayPoint)) 5.0 false
    (:OnSuccess
      (Math|Integer|IncrementInt (Variables|Default|GetCurrentWayPoint)
        (:%20%20
          (if (>= (Variables|Default|GetCurrentWayPoint) (Utilities|Array|Length (Variables|Default|GetwayPoints)))
            (Variables|Default|SetCurrentWayPoint 0))
          (Utilities|FlowControl|Delay 1.0)
          (CallFunction|ChasePlayer))))))

(event EventBeginPlay
  (CallFunction|ChasePlayer))

(fn ConstructionScript)